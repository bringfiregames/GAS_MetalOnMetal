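; BP_Etasphera08_03 is a modular character Blueprint for Etasphera08, assembled from separate skeletal mesh parts for the arms, individual finger segments, body, hips, plasma head and legs.
; Its Construction Script sets Mesh as the leader pose component for every part, so they all follow one skeleton pose instead of animating separately.
; No gameplay logic is present beyond this pose linking.
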(fn ConstructionScript
  (Components|SkinnedMesh|SetLeaderPoseComponent (Variables|Default|GetSK_Etasphera08_Arm_thumb_03_l) (Variables|Character|GetMesh) false false))